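; Player character for hang gliding, which creates a stopwatch widget and adds the hang-gliding Enhanced Input mapping on BeginPlay.
; The angle input directly edits movement velocity, either building forward speed or trading it for a slight climb, within clamps.
; With neutral input, Tick bleeds forward speed toward a minimum and applies a steady sink.
; Jump and move handlers remain, alongside an unconnected falling-gravity check.
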(event Input|EnhancedActionEvents|EnhancedInputActionIA_Move
  (params (ActionValue :type Float%20%28double-precision%29) (ElapsedSeconds :type Float%20%28double-precision%29) (TriggeredSeconds :type Float%20%28double-precision%29) (InputAction :type Input%20Action%20Object%20Reference :default "/Game/Input/Actions/IA_Move.IA_Move"))
  ;[1 1 1] Unused Code
  (Pawn|Input|AddMovementInput "1.000000,0.000000,0.000000" ActionValue false))

(event Input|EnhancedActionEvents|EnhancedInputActionIA_Jump
  (params (ActionValue :type Boolean) (ElapsedSeconds :type Float%20%28double-precision%29) (TriggeredSeconds :type Float%20%28double-precision%29) (InputAction :type Input%20Action%20Object%20Reference :default "/Game/Input/Actions/IA_Jump.IA_Jump"))
  ;[1 1 1] Unused Code
  (:Started
    (Character|Jump))
  (:Completed
    (Character|StopJumping)))

(event Input|EnhancedActionEvents|EnhancedInputActionIA_Angle
  (params (ActionValue :type Float%20%28double-precision%29) (ElapsedSeconds :type Float%20%28double-precision%29) (TriggeredSeconds :type Float%20%28double-precision%29) (InputAction :type Input%20Action%20Object%20Reference :default "/Game/Input/Actions/IA_Angle.IA_Angle"))
  (bind _returnvalue (Transformation|GetVelocity))
  (bind _returnvalue_2 (Transformation|GetVelocity))
  (:Triggered
    (Variables|Default|SetIsNeutral false)
    (if (> ActionValue 0.0)
      (Variables|/Script/Engine.MovementComponent|SetVelocity (Variables|Character|GetCharacterMovement) (Math|Vector|MakeVector (Math|Conversions|ToFloat(Integer) (Class|KismetMathLibrary|ClampInt64 (Class|KismetMathLibrary|ToInt64(Float) (+ (.x _returnvalue) 5.0)) -9999 1000)) (.y _returnvalue) (Math|Conversions|ToFloat(Integer) (Class|KismetMathLibrary|ClampInt64 (Class|KismetMathLibrary|ToInt64(Float) (- (.z _returnvalue) -2.0)) -1000 9999))))
      (elif (< ActionValue 0.0)
        (Variables|/Script/Engine.MovementComponent|SetVelocity (Variables|Character|GetCharacterMovement) (Math|Vector|MakeVector (Math|Conversions|ToFloat(Integer) (Class|KismetMathLibrary|ClampInt64 (Class|KismetMathLibrary|ToInt64(Float) (- (.x _returnvalue_2) 1e+01)) 50 9999)) (.y _returnvalue_2) 1e+01)))))
  (:Completed
    (Variables|Default|SetIsNeutral true)))

(event EventBeginPlay
  (bind _returnvalue (UserInterface|CreateWidget "/Game/Blueprints/UW_Stopwatch.UW_Stopwatch_C"))
  (UserInterface|Viewport|AddtoViewport _returnvalue 0)
  (bind _asplayer_controller (Utilities|Casting|CastToPlayerController (Pawn|GetController)))
  (Input|AddMappingContext (PlayerController|LocalPlayerSubsystems|GetEnhancedInputLocalPlayerSubsystem _asplayer_controller) "/Game/Input/IMC_Hanggliding.IMC_Hanggliding" 0 "(bIgnoreAllPressedKeysUntilRelease=True,bForceImmediately=False,bNotifyUserSettings=False)")
  (Variables|Default|SetIsNeutral true))

(event Collision|EventActorBeginOverlap
  (params (OtherActor :type Actor%20Object%20Reference)))

(event EventTick
  (params (DeltaSeconds :type Float%20%28single-precision%29))
  (bind _returnvalue (Transformation|GetVelocity))
  (if (Variables|Default|GetIsNeutral)
    (Variables|/Script/Engine.MovementComponent|SetVelocity (Variables|Character|GetCharacterMovement) (Math|Vector|MakeVector (Math|Conversions|ToFloat(Integer) (Math|Conversions|ToInteger(Byte) (Class|KismetMathLibrary|ClampInt64 (Class|KismetMathLibrary|ToInt64(Float) (- (.x _returnvalue) 7.0)) 200 9999))) (.y _returnvalue) -5e+01))))

(fn ConstructionScript)