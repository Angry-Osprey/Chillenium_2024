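; Player Paper2D character for a hang-gliding game, steered with Enhanced Input and propelled by movement-component impulses.
; Tick pushes it forward with random lift and picks a flipbook from vertical speed, while angle, move and descend inputs adjust the flight.
; StartTimer creates the stopwatch widget.
; Hitting an actor named like "Test_level" shows game over, pauses the game and stops the stopwatch; respawn and velocity-clamp logic is disconnected.
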(event OnComponentHit(CapsuleComponent)
  (params (HitComponent :type Primitive%20Component%20Object%20Reference) (OtherActor :type Actor%20Object%20Reference) (OtherComp :type Primitive%20Component%20Object%20Reference) (NormalImpulse :type Vector :default "0, 0, 0") (Hit :type Hit%20Result%20Structure%20%28by%20ref%29))
  (bind _returnvalue (Game|GetPlayerController 0))
  (if (Utilities|String|Contains (Utilities|GetDisplayName OtherActor) "Test_level")
    (Variables|/Script/Engine.PlayerController|SetbShowMouseCursor _returnvalue true)
    (Input|SetInputModeUIOnly _returnvalue 0 "DoNotLock" false)
    (bind _returnvalue_2 (UserInterface|CreateWidget "/Game/Blueprints/UW_Gameover.UW_Gameover_C"))
    (UserInterface|Viewport|AddtoViewport _returnvalue_2 0)
    (Game|SetGamePaused true)
    (bind _asbp_player_ty (Utilities|Casting|CastToBP_PlayerTY (Game|GetPlayerCharacter 0)))
    (CallFunction|ToggleStopwatch _asbp_player_ty true)))

(event Custom|StartTimer
  (bind _returnvalue (UserInterface|CreateWidget "/Game/Blueprints/UW_Stopwatch.UW_Stopwatch_C"))
  (bind _output_get (Variables|Default|SetStopwatch_Widget _returnvalue))
  (UserInterface|Viewport|AddtoViewport _output_get 0))

(event Custom|CustomEvent_1
  (bind _returnvalue (UserInterface|CreateWidget "/Game/Blueprints/UW_Stopwatch.UW_Stopwatch_C"))
  (UserInterface|Viewport|AddtoViewport _returnvalue 0)
  (bind _asplayer_controller (Utilities|Casting|CastToPlayerController (Pawn|GetController)))
  (Input|AddMappingContext (PlayerController|LocalPlayerSubsystems|GetEnhancedInputLocalPlayerSubsystem _asplayer_controller) "/Game/Input/IMC_Hanggliding.IMC_Hanggliding" 0 "(bIgnoreAllPressedKeysUntilRelease=True,bForceImmediately=False,bNotifyUserSettings=False)")
  (Variables|Default|SetIsNeutral true))

(event Custom|CustomEvent
  (params (DeltaSeconds :type Float%20%28single-precision%29))
  (bind _sprite (Variables|Default|GetSprite))
  (if (> (Math|Vector|VectorLength (Math|Vector|MakeVector (.x (Transformation|GetVelocity)) 0.0 0.0)) 2.0)
    (Sprite|SetFlipbook _sprite "/Game/Player/fast_Char_1.fast_Char_1")
    (else
      (Sprite|SetFlipbook _sprite "/Game/Player/Idle_Char_1.Idle_Char_1"))))

(event Input|EnhancedActionEvents|EnhancedInputActionIA_Move
  (params (ActionValue :type Float%20%28double-precision%29) (ElapsedSeconds :type Float%20%28double-precision%29) (TriggeredSeconds :type Float%20%28double-precision%29) (InputAction :type Input%20Action%20Object%20Reference :default "/Game/Input/Actions/IA_Move.IA_Move"))
  ;[1 1 1] Unused Code
  (Pawn|Input|AddMovementInput "1.000000,0.000000,0.000000" ActionValue false))

(event Input|EnhancedActionEvents|EnhancedInputActionIA_Jump
  (params (ActionValue :type Boolean) (ElapsedSeconds :type Float%20%28double-precision%29) (TriggeredSeconds :type Float%20%28double-precision%29) (InputAction :type Input%20Action%20Object%20Reference :default "/Game/Input/Actions/IA_Jump.IA_Jump"))
  ;[1 1 1] Unused Code
  (:Triggered
    (Physics|AddImpulse (Variables|Character|GetCharacterMovement) "0.000000,0.000000,150.000000" false))
  (:Started
    (Character|Jump))
  (:Completed
    (Character|StopJumping)))

(event Input|EnhancedActionEvents|EnhancedInputActionIA_Angle
  (params (ActionValue :type Float%20%28double-precision%29) (ElapsedSeconds :type Float%20%28double-precision%29) (TriggeredSeconds :type Float%20%28double-precision%29) (InputAction :type Input%20Action%20Object%20Reference :default "/Game/Input/Actions/IA_Angle.IA_Angle"))
  (:Started
    (Variables|Default|SetIsNeutral false)
    (if (> ActionValue 0.0)
      (Physics|AddImpulse (Variables|Character|GetCharacterMovement) "200.000000,0.000000,-250.000000" false)
      (elif (< ActionValue 0.0)
        (if true
          (Physics|AddImpulse (Variables|Character|GetCharacterMovement) (Math|Vector|MakeVector -9e+02 0.0 0.0) false)))))
  (:Completed
    (Variables|Default|SetIsNeutral true)))

(event Input|EnhancedActionEvents|EnhancedInputActiondescend
  (params (ActionValue :type Boolean) (ElapsedSeconds :type Float%20%28double-precision%29) (TriggeredSeconds :type Float%20%28double-precision%29) (InputAction :type Input%20Action%20Object%20Reference :default "/Game/Input/Actions/descend.descend"))
  (Physics|AddImpulse (Variables|Character|GetCharacterMovement) "0.000000,0.000000,-90.000000" false))

(event Collision|EventActorBeginOverlap
  (params (OtherActor :type Actor%20Object%20Reference)))

(event EventDestroyed)

(event EventTick
  (params (DeltaSeconds :type Float%20%28single-precision%29))
  (if (> (Math|Vector|VectorLength (Math|Vector|MakeVector 0.0 0.0 (.z (Transformation|GetVelocity)))) 2.0)
    (Sprite|SetFlipbook (Variables|Default|GetSprite) "/Game/Player/fastAsccend_Char_1.fastAsccend_Char_1")
    (Physics|AddImpulse (Variables|Character|GetCharacterMovement) (Math|Vector|MakeVector 25.0 0.0 (Math|Random|RandomFloatinRange 1e+01 25.0)) false :!label _label)
    (elif true
      (Sprite|SetFlipbook (Variables|Default|GetSprite) "/Game/Player/decend_Char_1.decend_Char_1")
      (goto _label)
      (else
        (Sprite|SetFlipbook (Variables|Default|GetSprite) "/Game/Player/Idle_Char_1.Idle_Char_1")))))

(event EventBeginPlay
  (bind _asplayer_controller (Utilities|Casting|CastToPlayerController (Pawn|GetController)))
  (Input|AddMappingContext (PlayerController|LocalPlayerSubsystems|GetEnhancedInputLocalPlayerSubsystem _asplayer_controller) "/Game/Input/IMC_Hanggliding.IMC_Hanggliding" 0 "(bIgnoreAllPressedKeysUntilRelease=True,bForceImmediately=False,bNotifyUserSettings=False)")
  (Physics|AddImpulse (Variables|Character|GetCharacterMovement) (Math|Vector|MakeVector 205.0 0.0 0.0) false))

(fn ConstructionScript)

(fn ToggleStopwatch
  (params (isPaused :type Boolean))
  (Variables|/Game/Blueprints/UW_Stopwatch.UW_Stopwatch_C|SetisPaused (Variables|Default|GetStopwatch_Widget) isPaused))